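; Actor component that tracks its owner's health and reports hurt, heal and death through event dispatchers.
; On BeginPlay it fills health to maximum and binds to the owner's OnTakeAnyDamage.
; The damage handler clamps health and broadcasts the normalized value, treating zero or negative damage as healing.
; At zero health it broadcasts death and unbinds from further damage.
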(event EventBeginPlay
  (Variables|Health|SetCurrentHealth (Variables|Health|GetMaxHealth))
  (EventDispatchers|BindEventtoOnTakeAnyDamage (Components|GetOwner) (EventDispatchers|CreateEvent :!event HandleDamage)))

(event EventTick
  (params (DeltaSeconds :type Float%20%28single-precision%29)))

(fn HandleDamage
  (params (DamagedActor :type Actor%20Object%20Reference) (Damage :type Float%20%28single-precision%29) (DamageType :type Damage%20Type%20Object%20Reference) (InstigatedBy :type Controller%20Object%20Reference) (DamageCauser :type Actor%20Object%20Reference))
  (Variables|Health|SetCurrentHealth (Math|Float|Clamp(Float) (- (Variables|Health|GetCurrentHealth) Damage) 0.0 (Variables|Health|GetMaxHealth)))
  (if (> (Variables|Health|GetCurrentHealth) 0.0)
    (if (> Damage 0.0)
      (Default|CallOnHurt (/ (Variables|Health|GetCurrentHealth) (Variables|Health|GetMaxHealth)))
      (else
        (Default|CallOnHeal (/ (Variables|Health|GetCurrentHealth) (Variables|Health|GetMaxHealth)))))
    (else
      (Default|CallOnDeath 0.0)
      (EventDispatchers|UnbindEventfromOnTakeAnyDamage (Components|GetOwner) (EventDispatchers|CreateEvent :!event HandleDamage)))))