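; Projectile actor that applies damage to the first actor it overlaps, then destroys itself.
; On BeginPlay it caches its owner as the instigating Controller and starts a DestroyTime timer, printing an error if the owner is not a Controller.
; The Construction Script binds the sphere collision's begin-overlap, and HandleOverlap applies BaseDamage credited to that controller.
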(event EventBeginPlay
  (bind _ascontroller (Utilities|Casting|CastToController (Components|GetOwner))
    (:then
      (Variables|Default|SetOwnerController _ascontroller)
      (Utilities|Time|SetTimerbyEvent (EventDispatchers|CreateEvent :!event K2DestroyActor) (Variables|Default|GetDestroyTime)))
    (:CastFailed
      (Development|PrintString "Projectile: We need an owner to be a controller"))))

(event Collision|EventActorBeginOverlap
  (params (OtherActor :type Actor%20Object%20Reference)))

(event EventTick
  (params (DeltaSeconds :type Float%20%28single-precision%29)))

(fn ConstructionScript
  (Collision|BindEventtoOnComponentBeginOverlap (Variables|Default|GetSphereCollision_0) (EventDispatchers|CreateEvent :!event HandleOverlap)))

(fn HandleOverlap
  (params (OverlappedComponent :type Primitive%20Component%20Object%20Reference) (OtherActor :type Actor%20Object%20Reference) (OtherComp :type Primitive%20Component%20Object%20Reference) (OtherBodyIndex :type Integer) (bFromSweep :type Boolean) (SweepResult :type Hit%20Result%20Structure%20%28by%20ref%29))
  (Game|Damage|ApplyDamage OtherActor (Variables|Default|GetBase%20Damage) (Variables|Default|GetOwnerController) self)
  (Actor|DestroyActor)
  (return))