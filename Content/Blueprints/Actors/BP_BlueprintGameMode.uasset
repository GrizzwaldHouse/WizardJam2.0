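; Game mode that tracks the player and enemy count and holds the win and lose handling.
; BeginPlay scans BP_BaseCharacter actors, storing the BP_BasePlayer, binding its lost event and counting the rest as enemies.
; RemoveEnemy decrements the count and declares victory at zero; RemovePlayer shows defeat with UI-only input, both using a results widget.
; The enemy OnDestroyed binding and results widget creation are disconnected, so neither runs.
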(event EventBeginPlay
  (bind _outactors (Actor|GetAllActorsOfClass "/Game/Blueprints/Actors/BP_BaseCharacter.BP_BaseCharacter_C"))
  (for _array_element _outactors
    (bind _asbp_base_player (Utilities|Casting|CastToBP_BasePlayer _array_element)
      (:then
        (Variables|Default|SetCurrentPlayer _asbp_base_player)
        (EventDispatchers|BindEventtoOnPlayerLost _asbp_base_player (EventDispatchers|CreateEvent :!event RemovePlayer)))
      (:CastFailed
        (Math|Integer|IncrementInt (Variables|Default|GetNumberOfEnemies)))))
  (bind _returnvalue (Actor|GetActorOfClass (Variables|Default|GetPlayerControllerClass))))

(fn ConstructionScript)

(fn RemoveEnemy
  (params (DestroyedActor :type Actor%20Object%20Reference))
  (bind _resultswidgetobject (Variables|Default|GetResultsWidgetObject))
  (bind _result (Math|Integer|DecrementInt (Variables|Default|GetNumberOfEnemies))
    (:%20%20
      (if (not (> _result 0))
        (Development|PrintString "You Win!" true true "(R=0.391593,G=1.000000,B=0.307425,A=1.000000)" 12.0)
        (UserInterface|Viewport|AddtoViewport _resultswidgetobject 0)
        (Default|WinConditionMet _resultswidgetobject)
        (Default|PlayerWin (Variables|Default|GetCurrentPlayer))))))

(fn RemovePlayer
  (bind _resultswidgetobject (Variables|Default|GetResultsWidgetObject))
  (Development|PrintString "You Lose!!" true true "(R=1.000000,G=0.071981,B=0.111783,A=1.000000)" 12.0)
  (UserInterface|Viewport|AddtoViewport _resultswidgetobject 0)
  (Input|SetInputModeUIOnly (Widget|GetOwningPlayer _resultswidgetobject) _resultswidgetobject "LockAlways" false))