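; AI controller for an agent pawn that runs a behavior tree and feeds it perception results.
; On possession it calls the parent handler, then starts the behavior tree asset.
; The construction script binds to AI Perception target updates.
; The perception handler writes any successfully sensed actor to the player blackboard key, without filtering, and clears that key when sensing fails.
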(event EventPossess
  (params (PossessedPawn :type Pawn%20Object%20Reference))
  (|CallParentFunction PossessedPawn)
  (AI|RunBehaviorTree (Variables|Default|GetBTAsset)))

(fn ConstructionScript
  (EventDispatchers|BindEventtoOnTargetPerceptionUpdated (Variables|Default|GetAIPerception) (EventDispatchers|CreateEvent :!event HandlePerception)))

(fn HandlePerception
  (params (Actor :type Actor%20Object%20Reference) (Stimulus :type AI%20Stimulus%20Structure))
  (bind _blackboard (Variables|Default|GetBlackboard))
  (bind _player_key (Variables|Default|GetPlayer%20Key))
  (if (.bSuccessfullySensed (Utilities|Struct|BreakAIStimulus Stimulus))
    (AI|Components|Blackboard|SetValueasObject _blackboard _player_key Actor)
    (else
      (AI|Components|Blackboard|ClearValue _blackboard _player_key))))