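; BP_BasePlayer is the player-controlled character, layering input and HUD on a parent that supplies shared health handling.
; BeginPlay creates the HUD and binds weapon ammo and heal events, destroying the actor if controller or HUD is missing.
; Inputs drive yaw-relative movement, look, attack and reload through WeaponObject.
; Hurt and death overrides update HUD health, with death disabling input and collision; win and loss functions remove the HUD.
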(event EventBeginPlay
  (|CallParentFunction)
  (bind _asplayer_controller (Utilities|Casting|CastToPlayerController (Pawn|GetController))
    (:then
      (Variables|Default|SetPlayerController _asplayer_controller)
      (bind _returnvalue (UserInterface|CreateWidget (Variables|Default|GetHUDClass) _asplayer_controller))
      (bind _aswbp_player_hud (Utilities|Casting|CastToWBP_PlayerHUD _returnvalue)
        (:then
          (bind _output_get (Variables|Default|SetHUDObject _aswbp_player_hud))
          (UserInterface|Viewport|AddtoViewport _returnvalue 0)
          (EventDispatchers|BindEventtoOnAmmoChanged (Variables|Default|GetWeaponObject) (EventDispatchers|CreateEvent _output_get :!event SetAmmo))
          (Default|ReloadAmmo (Variables|Default|GetWeaponObject))
          (EventDispatchers|BindEventtoOnHeal (Variables|Default|GetHealthComponent) (EventDispatchers|CreateEvent (Variables|Default|GetHUDObject) :!event SetHealth)))
        (:CastFailed
          (Development|PrintString "Need HUD")
          (Actor|DestroyActor))))
    (:CastFailed
      (Development|PrintString "Failed to find Player Controller")
      (Actor|DestroyActor))))

(event Collision|EventActorBeginOverlap
  (params (OtherActor :type Actor%20Object%20Reference))
  (|CallParentFunction OtherActor) ; This node is disabled and will not be called.\nDrag off pins to build functionality.
)

(event EventTick
  (params (DeltaSeconds :type Float%20%28single-precision%29))
  (|CallParentFunction DeltaSeconds) ; This node is disabled and will not be called.\nDrag off pins to build functionality.
)

(event Input|ActionEvents|InputActionAttack
  (params (Key :type Key%20Structure :default "None"))
  ;[0.5625 0.1929 0 1 50] Input
  (:Pressed
    (Default|Attack (Variables|Default|GetWeaponObject))))

(event Input|ActionEvents|InputActionReload
  (params (Key :type Key%20Structure :default "None"))
  ;[0.5625 0.1929 0 1 50] Input
  (:Pressed
    (Default|RequestReload (Variables|Default|GetWeaponObject))))

(event Input|AxisEvents|InputAxisTurnRight
  (params (AxisValue :type Float%20%28single-precision%29))
  ;[0.5625 0.1929 0 1 50] Input
  (Pawn|Input|AddControllerYawInput AxisValue))

(event Input|AxisEvents|InputAxisMoveForward
  (params (AxisValue :type Float%20%28single-precision%29))
  ;[0.5625 0.1929 0 1 50] Input
  (Pawn|Input|AddMovementInput (Math|Vector|GetForwardVector (Math|Rotator|MakeRotator 0.0 0.0 (.Yaw (Math|Rotator|BreakRotator (Pawn|GetControlRotation :!class /Script/Engine.Pawn))))) AxisValue false))

(event Input|AxisEvents|InputAxisLookUp
  (params (AxisValue :type Float%20%28single-precision%29))
  ;[0.5625 0.1929 0 1 50] Input
  (Pawn|Input|AddControllerPitchInput AxisValue))

(event Input|AxisEvents|InputAxisMoveRight
  (params (AxisValue :type Float%20%28single-precision%29))
  ;[0.5625 0.1929 0 1 50] Input
  (Pawn|Input|AddMovementInput (Math|Vector|GetRightVector (Math|Rotator|MakeRotator 0.0 0.0 (.Yaw (Math|Rotator|BreakRotator (Pawn|GetControlRotation :!class /Script/Engine.Pawn))))) AxisValue false))

(fn ConstructionScript
  (|CallParentFunction))

(fn HandleHurt
  (params (Ratio :type Float%20%28double-precision%29))
  (|CallParentFunction Ratio)
  (Default|SetHealth (Variables|Default|GetHUDObject) Ratio))

(fn HandleDeath
  (params (Ratio :type Float%20%28double-precision%29))
  (|CallParentFunction Ratio)
  (Default|SetHealth (Variables|Default|GetHUDObject) 0.0)
  (Input|DisableInput (Variables|Default|GetPlayerController))
  (Collision|SetCollisionEnabled (Variables|Default|GetCapsuleComponent) "NoCollision"))

(fn CanPickHealth
  (return true))

(fn PlayerLost
  (Default|CallOnPlayerLost)
  (Variables|/Script/Engine.PlayerController|SetbShowMouseCursor (Variables|Default|GetPlayerController) true)
  (Widget|RemovefromParent (Variables|Default|GetHUDObject)))

(fn PlayerWin
  (Input|DisableInput (Variables|Default|GetPlayerController))
  (Widget|RemovefromParent (Variables|Default|GetHUDObject)))