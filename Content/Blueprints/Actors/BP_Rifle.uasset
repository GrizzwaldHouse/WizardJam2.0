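; Rifle actor that requires a parent Pawn and fires projectiles from its muzzle socket, with ammo and reload handling.
; Attack and reload share an action lock; firing also needs life and ammo, and starts a timer.
; A flagged hack aims shots at the first player HUD widget's destination for its owning pawn, otherwise using base aim rotation.
; Dispatchers announce attacks, reload starts, action stops and ammo changes, while a separate event refills ammo.
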(event Custom|ActionStopped
  (Variables|Default|SetActionHappening false)
  (Default|CallOnActionStopped))

(event Custom|ReloadAmmo
  (bind _maxammo (Variables|Default|GetMaxAmmo))
  (bind _output_get (Variables|Default|SetCurrentAmmo _maxammo))
  (Default|CallOnAmmoChanged _output_get _maxammo))

(event EventBeginPlay
  (|CallParentFunction)
  (bind _aspawn (Utilities|Casting|CastToPawn (Actor|GetParentActor))
    (:then
      (Variables|Default|SetParentPawn _aspawn))
    (:CastFailed
      (Development|PrintString "Need a pawn to own this Rifle" true true "(R=1.000000,G=0.697862,B=0.000000,A=1.000000)")
      (Actor|DestroyActor))))

(event Collision|EventActorBeginOverlap
  (params (OtherActor :type Actor%20Object%20Reference)))

(event EventTick
  (params (DeltaSeconds :type Float%20%28single-precision%29)))

(fn ConstructionScript)

(fn Attack
  (bind _parentpawn (Variables|Default|GetParentPawn))
  (if (CallFunction|CanShoot)
    (Game|SpawnActorfromClass (Variables|Default|GetProjectileClass) (Math|Transform|MakeTransform (CallFunction|GetSource) (CallFunction|HACKDONOTEXPOSETOCODE) "1.000000,1.000000,1.000000") "Undefined" "MultiplyWithRoot" (Pawn|GetController _parentpawn) _parentpawn)
    (Variables|Default|SetActionHappening true)
    (Utilities|Time|SetTimerbyEvent (EventDispatchers|CreateEvent :!event Custom|ActionStopped) (Variables|Default|GetTime))
    (Default|CallOnRifleAttack)
    (CallFunction|UseAmmo)))

(fn CanShoot
  (return (Math|Boolean|ANDBoolean (not (Variables|Default|GetActionHappening)) (Variables|Default|GetAlive?) (> (Variables|Default|GetCurrentAmmo) 0.0))))

(fn GetSource
  (return (Transformation|GetSocketLocation (Variables|Default|GetSK_Rifle) "MuzzleFlashSocket")))

(fn HACKDONOTEXPOSETOCODE
  (bind _foundwidgets (Widget|GetAllWidgetsOfClass "/Game/Both/WBP_PlayerHUD.WBP_PlayerHUD_C" false))
  (if (== (Class|UserWidget|GetOwningPlayerPawn (Utilities|Array|Get(acopy) _foundwidgets)) (Variables|Default|GetParentPawn))
    (return (Math|Rotator|MakeRotfromX (- (Default|GetDestination (Utilities|Array|Get(acopy) _foundwidgets)) (CallFunction|GetSource))))
    (else
      (return (Pawn|GetBaseAimRotation (Variables|Default|GetParentPawn))))))

(fn UseAmmo
  (bind _output_get (Variables|Default|SetCurrentAmmo (Math|Float|Max(Float) (- (Variables|Default|GetCurrentAmmo) 1.0) 0.0)))
  (Default|CallOnAmmoChanged _output_get (Variables|Default|GetMaxAmmo)))

(fn RequestReload
  (if (not (Variables|Default|GetActionHappening))
    (Variables|Default|SetActionHappening true)
    (Default|CallOnReloadStart)))